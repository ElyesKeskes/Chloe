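; ChloeHUD is the HUD Blueprint that creates and manages the game's main menu, decision overlay, in-game overlay and ending screen widgets.
; The main menu appears on BeginPlay when the game instance flags it, while events add or remove the others and pass in choice or ending data.
; Level transitions play a BlackScreen fade forward, calling LoadLevel on the game mode when finished, or in reverse, removing the widget afterwards.
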(event `self.ReceiveBeginPlay`
  (bind _chloegameinstance (`/Game/Blueprints/Global/BPL_GlobalGetters.GetChloeGameInstance`))
  (if (`/Game/Blueprints/Global/ChloeGameInstance.InMainMenu` _chloegameinstance)
    (bind _returnvalue (`|CreateWidget` "/Game/Blueprints/UI/W_MainMenu.W_MainMenu_C"))
    (bind _output_get (set `self.MainMenuUI` _returnvalue))
    (`UserWidget.AddToViewport` _output_get 0)))

(event `/Game/Blueprints/Global/Interfaces/BPI_GameState.EventDecision`
  (params (Choices :type "Array of /Game/Data/ChoiceData Structure (by ref)"))
  (bind _returnvalue (`|CreateWidget` "/Game/Blueprints/UI/W_DecisionOverlay.W_DecisionOverlay_C"))
  (bind _output_get (set `self.DecisionUI` _returnvalue))
  (`/Game/Blueprints/UI/W_DecisionOverlay.Initialize` _output_get Choices)
  (`UserWidget.AddToViewport` _output_get 0))

(event `RemoveDecisionUI`
  (set `PlayerController.bShowMouseCursor` false (`.ChloePlayerController` (`/Game/Blueprints/Global/BPL_GlobalGetters.GetChloePawn`)))
  (`Widget.RemoveFromParent` (`self.DecisionUI`)))

(event `RemovegameOverlayUI`
  (`Widget.RemoveFromParent` (`self.IngameOverlayUI`)))

(event `/Game/Blueprints/Global/Interfaces/BPI_GameState.EventEnding`
  (params (EndingData :type "/Game/Data/EndingData Structure"))
  (bind _returnvalue (`|CreateWidget` "/Game/Blueprints/UI/W_EndingUI.W_EndingUI_C"))
  (bind _output_get (set `self.EndingUI` _returnvalue))
  (`/Game/Blueprints/UI/W_EndingUI.Setup` _output_get EndingData_Name_7_2BA2CDA943E66FEB5CCB43A49821256E EndingData_Description_4_AE688C6E4D33F4B8D26FFAA41FEE8170)
  (`UserWidget.AddToViewport` _output_get 0))

(event `/Game/Blueprints/Global/Interfaces/BPI_GameState.EventStartInteractive`
  (bind _returnvalue (`|CreateWidget` "/Game/Blueprints/UI/W_IngameOverlay.W_IngameOverlay_C"))
  (bind _output_get (set `self.IngameOverlayUI` _returnvalue))
  (`UserWidget.AddToViewport` _output_get 0))

(event `LevelTransitionFadeToBlack`
  (bind _returnvalue (`|CreateWidget` "/Game/Blueprints/UI/BlackScreen.BlackScreen_C"))
  (bind _output_get (set `self.BlackScreen` _returnvalue))
  (`UserWidget.AddToViewport` _output_get 0)
  (bind _fade (`/Game/Blueprints/UI/BlackScreen.Fade` _output_get))
  (`UserWidget.PlayAnimation` _output_get _fade 0.0 1 "Forward" 1.0 false)
  (`UserWidget.BindToAnimationFinished` _output_get _fade (delegate `AnimationFinished`)))

(event `AnimationFinished`
  (bind _chloegamemode (`/Game/Blueprints/Global/BPL_GlobalGetters.GetChloeGameMode`))
  (`/Game/Blueprints/Global/ChloeGameMode.LoadLevel` _chloegamemode))

(event `LevelTransitionFadeOutOfBlack`
  (bind _returnvalue (`|CreateWidget` "/Game/Blueprints/UI/BlackScreen.BlackScreen_C"))
  (bind _output_get (set `self.BlackScreen` _returnvalue))
  (`UserWidget.AddToViewport` _output_get 0)
  (bind _fade (`/Game/Blueprints/UI/BlackScreen.Fade` _output_get))
  (`UserWidget.PlayAnimation` _output_get _fade 0.0 1 "Reverse" 1.0 false)
  (`UserWidget.BindToAnimationFinished` _output_get _fade (delegate `AnimationFinished2`)))

(event `AnimationFinished2`
  (`Widget.RemoveFromParent` (`self.BlackScreen`)))

(fn `UserConstructionScript`)