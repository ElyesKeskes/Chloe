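; Game mode that drives Chloe's branching story by playing the Level Sequence of the game instance's current StoryPath.
; When a sequence ends, its path-end type selects the next sequence, a level-change fade, interactive play, a HUD decision or an ending.
; TogglePawn swaps the player pawn with the BP_Amelia cutscene actor.
; Tick caches the sequence camera transform so a spawned CineCamera can blend into gameplay.
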(event `self.ReceiveBeginPlay`
  (bind _currentstorypath (`/Game/Blueprints/Global/ChloeGameInstance.CurrentStoryPath` (`self.ChloeGameInstance`)))
  (`|ExecutionSequence`
    (:`then_0`
      (bind _chloehud (`/Game/Blueprints/Global/BPL_GlobalGetters.GetChloeHUD`))
      (set `self.ChloeHUD` _chloehud)
      (bind _chloegameinstance (`/Game/Blueprints/Global/BPL_GlobalGetters.GetChloeGameInstance`))
      (set `self.ChloeGameInstance` _chloegameinstance)
      (bind _returnvalue (`GameplayStatics.GetActorOfClass` "/Game/Assets/MetaHumans/Amelia/BP_Amelia.BP_Amelia_C"))
      (set `self.ChloeCutsceneActor` _returnvalue)
      (bind _outactors (`GameplayStatics.GetAllActorsOfClassWithTag` "/Script/CinematicCamera.CineCameraActor" "StaticCamera"))
      (set `self.TransitionCamera` (`|GetArrayItem` _outactors))
      (if (`self.Fastforward`)
        (set `self.PlaybackSpeed` 5.0)
        (else
          (set `self.PlaybackSpeed` 1.0))))
    (:`then_1`
      (if (not (`/Game/Blueprints/Global/ChloeGameInstance.InMainMenu` (`self.ChloeGameInstance`)))
        (if (`/Game/Blueprints/Global/ChloeGameInstance.GameStarted` (`self.ChloeGameInstance`))
          (bind _chloehud_2 (`/Game/Blueprints/Global/BPL_GlobalGetters.GetChloeHUD`))
          (`/Game/Blueprints/Global/ChloeHUD.LevelTransitionFadeOutOfBlack` _chloehud_2))
        (`|ExecutionSequence`
          (:`then_0`
            (`KismetSystemLibrary.PrintString` (`KismetTextLibrary.Conv_TextToString` (`|FormatText` "StoryPath / ID: {ID} / PathEnd Type: {PathEndType} / NextStoryPathID: {NSP ID} / Description: {Description}" (break `/Game/Data/StoryPathData` _currentstorypath) (`|GetEnumeratorNameAsString` (`.Type_24_D710EE7D422A163B088FD0A573277246` (break `/Game/Data/PathEndData` (`.PathEnd_18_BF64790646CB9AE805647485C7054016` (break `/Game/Data/StoryPathData` _currentstorypath))))) (`.NextStoryPathID_21_75145EDB4CD235332690BCA01A7BC0E6` (break `/Game/Data/StoryPathData` _currentstorypath)) (`.Description_15_FF21BDB04BBBD2B63CA504AFDF50ED81` (break `/Game/Data/StoryPathData` _currentstorypath)))) true true (struct :`G` 1.0 :`B` 0.046007 :`A` 1.0) 20.0)
            (bind (_outactor _returnvalue_2) (`LevelSequencePlayer.CreateLevelSequencePlayer` (`.LevelSequence_2_786A136A4B9EB32C8730B1BEFD5CFB25` (break `/Game/Data/StoryPathData` _currentstorypath)) (make `MovieSceneSequencePlaybackSettings` false (make `MovieSceneSequenceLoopCount` 0) (struct :`bAllowRounding` true) (`self.PlaybackSpeed`) 0.0 false true true true false false "None" true)))
            (`/Engine/EditorBlueprintResources/StandardMacros.IsValid` _outactor
              (:`Is Valid`
                _)
              (:`Is Not Valid`
                (`KismetSystemLibrary.PrintString` "SEQUENCE INVALID" true true (struct :`R` 1.0 :`B` 0.005519 :`A` 1.0) 10.0)))
            (`/Engine/EditorBlueprintResources/StandardMacros.IsValid` _returnvalue_2
              (:`Is Valid`
                (set `self.LevelSequenceActor` _outactor)
                (set `self.LevelSequencePlayer` _returnvalue_2))
              (:`Is Not Valid`
                (`KismetSystemLibrary.PrintString` "SEQUENCE INVALID 2" true true (struct :`R` 1.0 :`B` 0.005519 :`A` 1.0) 10.0))))
          (:`then_1`
            (add `MovieSceneSequencePlayer.OnFinished` (`self.LevelSequencePlayer`) (delegate `HandleSequenceEnd`))
            (add `self.ProcessNextStoryPath` (delegate `ProcessNextStoryPath_Event`)))
          (:`then_2`
            (`MovieSceneSequencePlayer.Play` (`self.LevelSequencePlayer`))
            (`self.TogglePawn` false)
            (set `/Game/Blueprints/Global/ChloeGameInstance.GameStarted` true (`self.ChloeGameInstance`))))
        (else
          (`PlayerController.SetViewTargetWithBlend` (`.ChloePlayerController` (`/Game/Blueprints/Global/BPL_GlobalGetters.GetChloePawn`)) (`self.TransitionCamera`) 0.0 "VTBlend_Linear" 0.0 false))))))

(event `self.ReceiveTick`
  (params (DeltaSeconds :type "Float (single-precision)"))
  (bind _levelsequenceplayer (`self.LevelSequencePlayer`))
  (bind _returnvalue (`LevelSequencePlayer.GetActiveCameraComponent` _levelsequenceplayer))
  (`/Engine/EditorBlueprintResources/StandardMacros.IsValid` _levelsequenceplayer
    (:`Is Valid`
      (if (and (`MovieSceneSequencePlayer.IsPlaying` _levelsequenceplayer) (`/Game/Blueprints/Global/ChloeGameInstance.GameStarted` (`self.ChloeGameInstance`)))
        (`/Engine/EditorBlueprintResources/StandardMacros.IsValid` _returnvalue
          (:`Is Valid`
            (set `self.LastSequenceCameraActiveTransform` (`SceneComponent.K2_GetComponentToWorld` _returnvalue))))))))

(event `/Game/Blueprints/Global/Interfaces/BPI_GameState.EventChoiceMade`
  (params (ChoiceData :type "/Game/Data/ChoiceData Structure"))
  (`/Game/Blueprints/Global/ChloeHUD.RemoveDecisionUI` (`self.ChloeHUD`))
  (set `/Game/Blueprints/Global/ChloeGameInstance.CurrentStoryPath` (`|GetArrayItem` (`/Game/Blueprints/Global/ChloeGameInstance.StoryPaths` (`self.ChloeGameInstance`)) (- ChoiceData_StoryPathID_11_9D57F272442DEA943614AEAAA11F8043 1)) (`self.ChloeGameInstance`))
  (`self.ProcessNextStoryPath`))

(event `HandleSequenceEnd`
  (bind (_currentstorypath_id _currentstorypath_description _currentstorypath_levelsequence _currentstorypath_pathend) (break `/Game/Data/StoryPathData` (`/Game/Blueprints/Global/ChloeGameInstance.CurrentStoryPath` (`self.ChloeGameInstance`))))
  (switch `/Game/Data/PathEndingType` (`.Type_24_D710EE7D422A163B088FD0A573277246` (break `/Game/Data/PathEndData` _currentstorypath_pathend)) :!label _label
    (:`NewEnumerator0`
      (`self.HandleNextSequencePathEnd`))
    (:`NewEnumerator1`
      (`self.HandleLoadLevelPathEnd`))
    (:`NewEnumerator2`
      (`self.HandleInteractivePathEnd`)
      (`self.CameraTransitionToInteractive`)
      (`KismetSystemLibrary.Delay` 1.0)
      (`self.K2_DestroyActor` (`self.TransitionCamera`)))
    (:`NewEnumerator3`
      (`self.HandleDecisionPathEnd`))
    (:`NewEnumerator4`
      (`self.HandleEndingPathEnd`))))

(event `/Game/Blueprints/Global/Interfaces/BPI_GameState.EventSequencePathEnd`
  (`MovieSceneSequencePlayer.Pause` (`self.LevelSequencePlayer`))
  (goto _label))

(event `ProcessNextStoryPath_Event`
  (bind _levelsequenceactor (`self.LevelSequenceActor`))
  (bind _currentstorypath (`/Game/Blueprints/Global/ChloeGameInstance.CurrentStoryPath` (`self.ChloeGameInstance`)))
  (`KismetSystemLibrary.PrintString` (`KismetTextLibrary.Conv_TextToString` (`|FormatText` "StoryPath / ID: {ID} / PathEnd Type: {PathEndType} / NextStoryPathID: {NSP ID} / Description: {Description}" (break `/Game/Data/StoryPathData` _currentstorypath) (`|GetEnumeratorNameAsString` (`.Type_24_D710EE7D422A163B088FD0A573277246` (break `/Game/Data/PathEndData` (`.PathEnd_18_BF64790646CB9AE805647485C7054016` (break `/Game/Data/StoryPathData` _currentstorypath))))) (`.NextStoryPathID_21_75145EDB4CD235332690BCA01A7BC0E6` (break `/Game/Data/StoryPathData` _currentstorypath)) (`.Description_15_FF21BDB04BBBD2B63CA504AFDF50ED81` (break `/Game/Data/StoryPathData` _currentstorypath)))) true true (struct :`G` 1.0 :`B` 0.136314 :`A` 1.0) 20.0)
  (`self.TogglePawn` false)
  (`LevelSequenceActor.SetSequence` _levelsequenceactor (`.LevelSequence_2_786A136A4B9EB32C8730B1BEFD5CFB25` (break `/Game/Data/StoryPathData` _currentstorypath)))
  (`MovieSceneSequencePlayer.SetPlayRate` (`LevelSequenceActor.SequencePlayer` _levelsequenceactor) (`self.PlaybackSpeed`))
  (`MovieSceneSequencePlayer.Play` (`self.LevelSequencePlayer`))
  (`KismetSystemLibrary.Delay` 0.2)
  (bind _returnvalue (`GameplayStatics.GetActorOfClass` "/Game/Assets/MetaHumans/Amelia/BP_Amelia.BP_Amelia_C"))
  (set `self.ChloeCutsceneActor` _returnvalue))

(event `LoadLevel`
  (`GameplayStatics.OpenLevel` (`self.Level Name to Load`)))

(fn `CameraTransitionToInteractive`
  (bind (_chloepawn _chloecontroller _chloeplayercontroller) (`/Game/Blueprints/Global/BPL_GlobalGetters.GetChloePawn`))
  (bind _returnvalue (`|SpawnActorFromClass` "/Script/CinematicCamera.CineCameraActor" (`self.LastSequenceCameraActiveTransform`) "Undefined" "MultiplyWithRoot" null null))
  (bind _output_get (set `self.TransitionCamera` _returnvalue))
  (`PlayerController.SetViewTargetWithBlend` _chloeplayercontroller _output_get 0.0 "VTBlend_Linear" 0.0 false)
  (`PlayerController.SetViewTargetWithBlend` _chloeplayercontroller _chloepawn 1.0 "VTBlend_Linear" 0.0 false))

(fn `HandleDecisionPathEnd`
  (bind (_currentstorypath_id _currentstorypath_description _currentstorypath_levelsequence _currentstorypath_pathend) (break `/Game/Data/StoryPathData` (`/Game/Blueprints/Global/ChloeGameInstance.CurrentStoryPath` (`self.ChloeGameInstance`))))
  (message `/Game/Blueprints/Global/Interfaces/BPI_GameState.EventDecision` (`self.ChloeHUD`) (`.Choices_11_8E18D4144E7F9E56C498D486C94ADF8C` (break `/Game/Data/StoryDecisionData` (`.StoryDecision_21_FAAE8C2A4AFABFBE6B97C1929DCF9C8D` (break `/Game/Data/PathEndData` _currentstorypath_pathend)))))
  (`KismetSystemLibrary.PrintString` "DECISION PATH END" true true (struct :`R` 1.0 :`B` 0.678156 :`A` 1.0) 5.0))

(fn `HandleEndingPathEnd`
  (bind (_currentstorypath_id _currentstorypath_description _currentstorypath_levelsequence _currentstorypath_pathend) (break `/Game/Data/StoryPathData` (`/Game/Blueprints/Global/ChloeGameInstance.CurrentStoryPath` (`self.ChloeGameInstance`))))
  (message `/Game/Blueprints/Global/Interfaces/BPI_GameState.EventEnding` (`self.ChloeHUD`) (`.Ending_19_8F89CCBA4D3D0D213EA231A3290B5075` (break `/Game/Data/PathEndData` _currentstorypath_pathend)))
  (`KismetSystemLibrary.PrintString` "ENDING PATH END" true true (struct :`R` 1.0 :`B` 0.678156 :`A` 1.0) 5.0))

(fn `HandleInteractivePathEnd`
  (bind (_currentstorypath_id _currentstorypath_description _currentstorypath_levelsequence _currentstorypath_pathend _currentstorypath_nextstorypathid) (break `/Game/Data/StoryPathData` (`/Game/Blueprints/Global/ChloeGameInstance.CurrentStoryPath` (`self.ChloeGameInstance`))))
  (`|ExecutionSequence`
    (:`then_0`
      (`MovieSceneSequencePlayer.GoToEndAndStop` (`self.LevelSequencePlayer`)))
    (:`then_1`
      (`self.TogglePawn` true)
      (message `/Game/Blueprints/Global/Interfaces/BPI_GameState.EventStartInteractive` (`self.ChloeHUD`))
      (set `/Game/Blueprints/Global/ChloeGameInstance.CurrentStoryPath` (`|GetArrayItem` (`/Game/Blueprints/Global/ChloeGameInstance.StoryPaths` (`self.ChloeGameInstance`)) (- _currentstorypath_nextstorypathid 1)) (`self.ChloeGameInstance`))
      (`KismetSystemLibrary.PrintString` "INTERACTIVE PATH END" true true (struct :`R` 1.0 :`B` 0.678156 :`A` 1.0) 5.0))))

(fn `HandleLoadLevelPathEnd`
  (bind (_currentstorypath_id _currentstorypath_description _currentstorypath_levelsequence _currentstorypath_pathend _currentstorypath_nextstorypathid) (break `/Game/Data/StoryPathData` (`/Game/Blueprints/Global/ChloeGameInstance.CurrentStoryPath` (`self.ChloeGameInstance`))))
  (set `self.Level Name to Load` (`.LevelNameToLoad_18_17D14A584CA127002A56CF80253F98EC` (break `/Game/Data/PathEndData` _currentstorypath_pathend)))
  (set `/Game/Blueprints/Global/ChloeGameInstance.CurrentStoryPath` (`|GetArrayItem` (`/Game/Blueprints/Global/ChloeGameInstance.StoryPaths` (`self.ChloeGameInstance`)) (- _currentstorypath_nextstorypathid 1)) (`self.ChloeGameInstance`))
  (`KismetSystemLibrary.PrintString` "LOAD LEVEL PATH END" true true (struct :`R` 1.0 :`B` 0.678156 :`A` 1.0) 5.0)
  (bind _chloehud (`/Game/Blueprints/Global/BPL_GlobalGetters.GetChloeHUD`))
  (`/Game/Blueprints/Global/ChloeHUD.LevelTransitionFadeToBlack` _chloehud))

(fn `HandleNextSequencePathEnd`
  (bind (_currentstorypath_id _currentstorypath_description _currentstorypath_levelsequence _currentstorypath_pathend _currentstorypath_nextstorypathid) (break `/Game/Data/StoryPathData` (`/Game/Blueprints/Global/ChloeGameInstance.CurrentStoryPath` (`self.ChloeGameInstance`))))
  (set `/Game/Blueprints/Global/ChloeGameInstance.CurrentStoryPath` (`|GetArrayItem` (`/Game/Blueprints/Global/ChloeGameInstance.StoryPaths` (`self.ChloeGameInstance`)) (- _currentstorypath_nextstorypathid 1)) (`self.ChloeGameInstance`))
  (`self.ProcessNextStoryPath`)
  (`KismetSystemLibrary.PrintString` "NEXT SEQUENCE PATH END" true true (struct :`R` 1.0 :`B` 0.678156 :`A` 1.0) 5.0))

(fn `TogglePawn`
  (params (State :type Boolean))
  (bind (_chloepawn _chloecontroller _chloeplayercontroller) (`/Game/Blueprints/Global/BPL_GlobalGetters.GetChloePawn`))
  (bind (_chloepawn_2 _chloecontroller_2 _chloeplayercontroller_2) (`/Game/Blueprints/Global/BPL_GlobalGetters.GetChloePawn`))
  (bind _chloecutsceneactor (`self.ChloeCutsceneActor`))
  (if State
    (`self.SetActorHiddenInGame` (`self.ChloeCutsceneActor`) true)
    (`self.SetActorHiddenInGame` _chloepawn_2 false)
    (`self.EnableInput` _chloepawn_2 _chloeplayercontroller_2)
    (else
      (`/Engine/EditorBlueprintResources/StandardMacros.IsValid` _chloecutsceneactor
        (:`Is Valid`
          (`self.SetActorHiddenInGame` _chloecutsceneactor false))
        (:`Is Not Valid`
          _))
      (`self.SetActorHiddenInGame` _chloepawn true)
      (`self.DisableInput` _chloepawn _chloeplayercontroller))))

(fn `UserConstructionScript`)