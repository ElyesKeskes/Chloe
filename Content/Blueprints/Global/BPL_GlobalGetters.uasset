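; Blueprint function library of global getters for Chloe's project-specific HUD, GameInstance, GameMode and pawn.
; The HUD is reached through player 0's pawn, PlayerState and controller, then cast like the GameInstance and GameMode.
; The pawn getter finds the Chloe actor by class and also returns its controller and player controller 0.
; Failed casts or an invalid pawn print a red error message.
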(fn `GetChloeGameInstance`
  (returns (ChloeGameInstance :type "/Game/Blueprints/Global/ChloeGameInstance Object Reference"))
  (bind _aschloe_game_instance (cast `/Game/Blueprints/Global/ChloeGameInstance` (`GameplayStatics.GetGameInstance` null))
    (:`then`
      (return _aschloe_game_instance))
    (:`CastFailed`
      (`KismetSystemLibrary.PrintString` null "Could not cast GameInstance" true true (struct :`R` 1.0 :`G` 0.05927 :`A` 1.0)))))

(fn `GetChloeGameMode`
  (returns (ChloeGameMode :type "/Game/Blueprints/Global/ChloeGameMode Object Reference"))
  (bind _aschloe_game_mode (cast `/Game/Blueprints/Global/ChloeGameMode` (`GameplayStatics.GetGameMode` null))
    (:`then`
      (return _aschloe_game_mode))
    (:`CastFailed`
      (`KismetSystemLibrary.PrintString` null "Could not cast GameMode" true true (struct :`R` 1.0 :`G` 0.05927 :`A` 1.0)))))

(fn `GetChloeHUD`
  (returns (ChloeHUD :type "/Game/Blueprints/Global/ChloeHUD Object Reference"))
  (bind _aschloe_hud (cast `/Game/Blueprints/Global/ChloeHUD` (`PlayerController.GetHUD` (`PlayerState.GetPlayerController` (`Pawn.PlayerState` (`GameplayStatics.GetPlayerPawn` null)))))
    (:`then`
      (return _aschloe_hud))
    (:`CastFailed`
      (`KismetSystemLibrary.PrintString` null "Could not cast HUD" true true (struct :`R` 1.0 :`G` 0.05927 :`A` 1.0)))))

(fn `GetChloePawn`
  (returns (ChloePawn :type "/Game/Chloe Object Reference") (ChloeController :type "Controller Object Reference") (ChloePlayerController :type "PlayerController Object Reference"))
  (bind _returnvalue (`GameplayStatics.GetActorOfClass` null "/Game/Chloe.Chloe_C"))
  (`/Engine/EditorBlueprintResources/StandardMacros.IsValid` _returnvalue
    (:`Is Valid`
      (return _returnvalue (`Pawn.GetController` _returnvalue) (`GameplayStatics.GetPlayerController` _returnvalue)))
    (:`Is Not Valid`
      (`KismetSystemLibrary.PrintString` null "Could not cast Pawn" true true (struct :`R` 1.0 :`G` 0.05927 :`A` 1.0)))))