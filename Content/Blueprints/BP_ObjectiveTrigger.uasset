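; An objective trigger actor that advances a chain of objectives, and optionally the story path, when a Pawn overlaps it.
; Active state gates the overlap and controls a widget's visibility, with triggers flagged active switching on at BeginPlay.
; On overlap it activates the linked next trigger and deactivates itself, either playing a voiceline or, if TriggerNextPath is set, destroying itself and telling the Chloe game mode to process the next story event and hide active triggers.
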(event `Activate`
  (set `self.Active` true)
  (`SceneComponent.SetVisibility` (`self.Widget`) true false))

(event `Deactivate`
  (set `self.Active` false)
  (`SceneComponent.SetVisibility` (`self.Widget`) false false))

(event `self.ReceiveBeginPlay`
  (if (`self.Active`)
    (`self.Activate`)))

(event `self.ReceiveActorBeginOverlap`
  (params (OtherActor :type "Actor Object Reference"))
  (if (`GameplayStatics.ObjectIsA` OtherActor "/Script/Engine.Pawn")
    (if (`self.Active`)
      (`/Engine/EditorBlueprintResources/StandardMacros.IsValid` (`self.NextObjectiveTrigger`)
        (:`Is Valid`
          (`self.Activate` (`self.NextObjectiveTrigger`)))
        (:`Is Not Valid`
          _))
      (if (`self.TriggerNextPath`)
        (bind _chloegamemode (`/Game/Blueprints/Global/BPL_GlobalGetters.GetChloeGameMode`))
        (`self.Deactivate`)
        (`self.K2_DestroyActor` self)
        (`/Game/Blueprints/Global/ChloeGameMode.ProcessNextStoryPath_Event` _chloegamemode)
        (`/Game/Blueprints/Global/ChloeGameMode.HideActiveObjectiveTriggers` _chloegamemode)
        (else
          (`GameplayStatics.PlaySound2D` (`self.Voiceline`) 1.0 1.0 0.0 null null)
          (`self.Deactivate`))))))

(fn `UserConstructionScript`)